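; Bullet is a projectile actor that is launched by a physics impulse on its Sphere and deals damage to Enemy actors.
; Initialize sets its material, parent and damage, then pushes it along the given direction scaled by Speed.
; On overlap it ignores actors of the parent's class, damages Enemies, and destroys itself except against non-Enemy StoneGolems.
; Tick looks up the Player every frame and destroys the bullet beyond a fixed distance.
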(event `Initialize`
  (params (Material :type "Material Object Reference") (Parent :type "Actor Object Reference") (Direction :type "Vector Structure") (Damage :type "Float (double-precision)"))
  (bind _sphere (`self.Sphere`))
  (`PrimitiveComponent.SetMaterial` _sphere 0 Material)
  (set `self.Parent` Parent)
  (`PrimitiveComponent.AddImpulse` _sphere (* Direction (`self.Speed`)) "None" false)
  (set `self.Damage` Damage))

(event `self.Sphere.OnComponentBeginOverlap`
  (params (OverlappedComponent :type "PrimitiveComponent Object Reference") (OtherActor :type "Actor Object Reference") (OtherComp :type "PrimitiveComponent Object Reference") (OtherBodyIndex :type Integer) (bFromSweep :type Boolean) (SweepResult :type "HitResult Structure (by ref)"))
  (bind _returnvalue (`ActorComponent.GetOwner` (`Actor.RootComponent` OtherActor)))
  (if (`KismetSystemLibrary.IsValid` OtherActor)
    (if (not (== (`GameplayStatics.GetObjectClass` (`self.Parent`)) (`GameplayStatics.GetObjectClass` _returnvalue)))
      (bind _asenemy (cast `/Game/IBeWitching/Blueprints/Enemy` _returnvalue :!label _label)
        (:`then`
          (`/Game/IBeWitching/Blueprints/Enemy.TakeDamage` _asenemy (`self.Damage`)))
        (:`CastFailed`
          (cast `/Game/IBeWitching/Blueprints/StoneGolem` _returnvalue
            (:`CastFailed`
              _))))
      (`self.K2_DestroyActor`))
    (else
      (goto _label))))

(event `self.ReceiveTick`
  (params (DeltaSeconds :type "Float (single-precision)"))
  ;[0 0.8612 1] Tick
  (bind _returnvalue (`GameplayStatics.GetActorOfClass` "/Game/IBeWitching/Blueprints/Player.Player_C"))
  (if (> (`KismetMathLibrary.Vector_Distance` (`SceneComponent.K2_GetComponentLocation` (`Character.Mesh` _returnvalue)) (`SceneComponent.K2_GetComponentLocation` (`self.Sphere`))) 1000.0)
    (`self.K2_DestroyActor`)))

(fn `UserConstructionScript`)