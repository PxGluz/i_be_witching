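; Player character with health, death, respawn, Enhanced Input movement and cooldown-limited shooting toward the cursor.
; Cursor rays projected onto the Z=0 plane aim bullets and position a placement hologram.
; Placing mode blocks movement, edge-scrolls the camera and spawns the chosen actor on click if the hologram shows its valid material, initializing planting grounds.
; Health drives the UI bar; death shows game over and halves the TouchStone's stored amounts.
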(event `Respawn`
  ;[1 0 0] Respawn Function
  (`SceneComponent.K2_SetWorldLocation` (`self.CapsuleComponent`) (`self.SpawnLocation`) false false)
  (set `self.CurrentHealth` (`self.MaxHealth`))
  (`/Game/IBeWitching/Blueprints/PlayerUI.GameOverScreen` (`self.PlayerUI`) false)
  (set `self.Dead` false)
  (`SkeletalMeshComponent.PlayAnimation` (`self.Mesh`) "/Game/IBeWitching/Animations/DieRecoverAnim.DieRecoverAnim" false))

(event `Die`
  ;[1 0 0] Death Function
  (set `self.Dead` true)
  (`/Game/IBeWitching/Blueprints/PlayerUI.GameOverScreen` (`self.PlayerUI`) true)
  (`SkeletalMeshComponent.PlayAnimation` (`self.Mesh`) "/Game/IBeWitching/Animations/DieAnim.DieAnim" false)
  (bind _returnvalue (`GameplayStatics.GetActorOfClass` "/Game/IBeWitching/Blueprints/TouchStone.TouchStone_C"))
  (bind _storage (`/Game/IBeWitching/Blueprints/TouchStone.Storage` _returnvalue))
  (for (_array_element _array_index) _storage
    (`KismetArrayLibrary.Array_Set` _storage _array_index (/ _array_element 2))))

(event `TakeDamage`
  (params (Amount :type "Float (double-precision)"))
  (bind _returnvalue (- (`self.CurrentHealth`) Amount))
  ;[1 0 0.006631] Take Damage Function
  (if (<= _returnvalue 0.0)
    (set `self.CurrentHealth` 0.0)
    (if (not (`self.Dead`))
      (`self.Die`))
    (else
      (set `self.CurrentHealth` _returnvalue))))

(event `Heal`
  (params (Amount :type "Float (double-precision)"))
  (bind _maxhealth (`self.MaxHealth`))
  (bind _returnvalue (+ Amount (`self.CurrentHealth`)))
  ;[1 0 0] Heal Function
  (if (> _returnvalue _maxhealth)
    (set `self.CurrentHealth` _maxhealth)
    (else
      (set `self.CurrentHealth` _returnvalue))))

(event `self.ReceiveTick`
  (params (DeltaSeconds :type "Float (single-precision)"))
  (bind _maxhealth (`self.MaxHealth`))
  (bind _playercam (`self.PlayerCam`))
  (bind _hologram (`self.Hologram`))
  (bind _playercam_2 (`self.PlayerCam`))
  (bind _returnvalue (`SceneComponent.K2_GetComponentLocation` _playercam))
  (bind (_worldlocation _worlddirection) (`PlayerController.DeprojectMousePositionToWorld` (`GameplayStatics.GetPlayerController` 0)))
  (bind _returnvalue_2 (`SceneComponent.K2_GetComponentLocation` _playercam_2))
  (bind _health (`/Game/IBeWitching/Blueprints/PlayerUI.Health` (`self.PlayerUI`)))
  (bind _returnvalue_3 (`WidgetLayoutLibrary.SlotAsCanvasSlot` _health))
  (bind (_returnvalue_x _returnvalue_y) (`KismetMathLibrary.BreakVector2D` (`CanvasPanelSlot.GetSize` _returnvalue_3)))
  ;[0 0.7772 1] Tick
  (`CanvasPanelSlot.SetSize` _returnvalue_3 (`KismetMathLibrary.MakeVector2D` _maxhealth _returnvalue_y))
  (set `ProgressBar.Percent` (/ (`self.CurrentHealth`) _maxhealth) _health)
  (if (`self.PlacingMode`)
    (`SceneComponent.K2_SetWorldTransform` _hologram (`KismetMathLibrary.MakeTransform` (+ _worldlocation (* (* _worlddirection (/ (.z _worldlocation) (.z _worlddirection))) (-1.0 -1.0 -1.0)))) false false)
    (bind _returnvalue_4 (`WidgetLayoutLibrary.GetMousePositionOnViewport`))
    (bind (_x _y) (`KismetMathLibrary.BreakVector2D` (/ _returnvalue_4 (`WidgetLayoutLibrary.GetViewportSize`))))
    (if (<= _x 0.05)
      (`SceneComponent.K2_SetWorldLocation` _playercam (+ _returnvalue (0.0 -5.0 0.0)) false false)
      (elif (>= _x 0.95)
        (`SceneComponent.K2_SetWorldLocation` _playercam (+ _returnvalue (0.0 5.0 0.0)) false false)))
    (if (<= _y 0.05)
      (`SceneComponent.K2_SetWorldLocation` _playercam_2 (+ _returnvalue_2 (5.0 0.0 0.0)) false false)
      (elif (>= _y 0.95)
        (`SceneComponent.K2_SetWorldLocation` _playercam_2 (+ _returnvalue_2 (-5.0 0.0 0.0)) false false)))
    (else
      (`SceneComponent.K2_SetRelativeLocation` (`self.PlayerCam`) (`self.CameraInitPos`) false false)
      (`SceneComponent.K2_SetWorldLocation` _hologram (0.0 0.0 -2000.0) false false))))

(event `self.ReceiveBeginPlay`
  ;[0 0.9148 1] Initializations
  (bind _asplayer_controller (cast `PlayerController` (`self.GetController`)))
  (bind _returnvalue (pcsubsystem `EnhancedInputLocalPlayerSubsystem` _asplayer_controller))
  (`/Engine/EditorBlueprintResources/StandardMacros.IsValid` _returnvalue
    (:`Is Valid`
      (`EnhancedInputSubsystemInterface.AddMappingContext` _returnvalue "/Game/IBeWitching/Actions/MyInputContext.MyInputContext" 0 (struct))
      (set `self.SpawnLocation` (`SceneComponent.K2_GetComponentLocation` (`self.CapsuleComponent`)))
      (bind _returnvalue_2 (`|CreateWidget` "/Game/IBeWitching/Blueprints/PlayerUI.PlayerUI_C" (`GameplayStatics.GetPlayerController` 0)))
      (bind _output_get (set `self.PlayerUI` _returnvalue_2))
      (`UserWidget.AddToViewport` _output_get 0)
      (set `PlayerController.bShowMouseCursor` true (`GameplayStatics.GetPlayerController` 0))
      (`/Game/IBeWitching/Blueprints/PlayerUI.GameOverScreen` (`self.PlayerUI`) false)
      (set `self.CameraInitPos` (`SceneComponent.RelativeLocation` (`self.PlayerCam`))))))

(event `EnhancedInput|/Game/IBeWitching/Actions/MyMove`
  (params (ActionValue :type "Vector2D Structure") (ElapsedSeconds :type "Float (double-precision)") (TriggeredSeconds :type "Float (double-precision)") (InputAction :type "InputAction Object Reference" :default "/Game/IBeWitching/Actions/MyMove.MyMove"))
  (bind (_returnvalue_roll _returnvalue_pitch _returnvalue_yaw) (`KismetMathLibrary.BreakRotator` (`self.GetControlRotation`)))
  (bind (_returnvalue_roll_2 _returnvalue_pitch_2 _returnvalue_yaw_2) (`KismetMathLibrary.BreakRotator` (`self.GetControlRotation`)))
  (bind _mesh (`self.Mesh`))
  (bind (_returnvalue_x _returnvalue_y) (`KismetMathLibrary.BreakVector2D` (* ActionValue (`self.Speed`))))
  (bind _returnvalue (and (not (`self.Dead`)) (not (`self.UIOpen`)) (not (`self.PlacingMode`))))
  ;[1 0.3726 0] Movement Handling
  (:`Triggered`
    (if _returnvalue
      (`self.AddMovementInput` (`KismetMathLibrary.GetRightVector` (`KismetMathLibrary.MakeRotator` _returnvalue_roll_2 0.0 _returnvalue_yaw_2)) _returnvalue_x)
      (`self.AddMovementInput` (`KismetMathLibrary.GetForwardVector` (`KismetMathLibrary.MakeRotator` 0.0 0.0 _returnvalue_yaw)) _returnvalue_y)))
  (:`Started`
    (if _returnvalue
      ;;[1 1 1] Animation Logic
      (`SkeletalMeshComponent.PlayAnimation` _mesh "/Game/IBeWitching/Animations/BattleRunForwardAnim.BattleRunForwardAnim" true)))
  (:`Completed`
    (if _returnvalue
      (`SkeletalMeshComponent.PlayAnimation` _mesh "/Game/IBeWitching/Animations/Idle02Anim.Idle02Anim" true))))

(event `Key|LeftMouseButton`
  (params (Key :type "Key Structure"))
  (bind (_returnvalue_location _returnvalue_rotation _returnvalue_scale) (`KismetMathLibrary.BreakTransform` (`SceneComponent.K2_GetComponentToWorld` (`self.CapsuleComponent`))))
  (bind (_worldlocation _worlddirection) (`PlayerController.DeprojectMousePositionToWorld` (`GameplayStatics.GetPlayerController` 0)))
  ;[1 0.3755 0] Shooting
  (:`Pressed`
    (if (`self.PlacingMode`)
      (for _array_element (`SceneComponent.GetChildrenComponents` (`self.Hologram`) true)
        (bind _asstatic_mesh_component (cast `StaticMeshComponent` _array_element)
          (:`then`
            (if (== "/Game/IBeWitching/Materials/HologramValid.HologramValid" (`PrimitiveComponent.GetMaterial` _asstatic_mesh_component 0))
              (bind _returnvalue (`|SpawnActorFromClass` (`self.ActorToBePlaced`) (`SceneComponent.K2_GetComponentToWorld` (`self.Hologram`)) "Undefined" "MultiplyWithRoot" null null))
              (bind _asplanting_gounds (cast `/Game/IBeWitching/Blueprints/PlantingGounds` _returnvalue)
                (:`then`
                  (`/Game/IBeWitching/Blueprints/PlantingGounds.Initialization` _asplanting_gounds (`self.PlantingGroundsPlant`)))
                (:`CastFailed`
                  _))
              (set `self.PlacingMode` false)
              (break)))
          (:`CastFailed`
            (`KismetSystemLibrary.PrintString` "Hello"))))
      (elif (and (`self.CanShoot`) (not (`self.Dead`)) (not (`self.UIOpen`)))
        (set `self.CanShoot` false)
        (bind _returnvalue_2 (`|SpawnActorFromClass` "/Game/IBeWitching/Blueprints/Bullet.Bullet_C" (`KismetMathLibrary.MakeTransform` _returnvalue_location _returnvalue_rotation _returnvalue_scale) "Undefined" "MultiplyWithRoot" null null))
        (`/Game/IBeWitching/Blueprints/Bullet.Initialize` _returnvalue_2 (`self.BulletMat`) self (`KismetMathLibrary.GetDirectionUnitVector` (`KismetMathLibrary.MakeVector` (.x _returnvalue_location) (.y _returnvalue_location)) (+ _worldlocation (* (* _worlddirection (/ (.z _worldlocation) (.z _worlddirection))) (-1.0 -1.0 -1.0)))) (`self.Damage`))
        (`KismetSystemLibrary.Delay` 0.5)
        (set `self.CanShoot` true)))))

(fn `UserConstructionScript`)