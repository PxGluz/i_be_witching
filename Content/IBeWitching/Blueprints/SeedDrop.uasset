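; SeedDrop is a floating text popup announcing that one seed of a given type was gained.
; Initialize sets the text render to the Shinykin, Ghostlilly or Bushbow seed label based on Type.
; Each tick, the text eases upward with a frame-based lerp and turns toward the player camera, ignoring the camera's Y offset.
; The actor destroys itself once the text rises past a height threshold.
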(event `Initialize`
  (params (Type :type Integer))
  (bind _textrender (`self.TextRender`))
  ;[0 0.9587 1] Initialization Function
  (switch `int` Type
    (:`0`
      (`TextRenderComponent.K2_SetText` _textrender (`KismetTextLibrary.Conv_StringToText` (`KismetStringLibrary.BuildString_Int` "" "+" 1 " Shinykin Seed"))))
    (:`1`
      (`TextRenderComponent.K2_SetText` _textrender (`KismetTextLibrary.Conv_StringToText` (`KismetStringLibrary.BuildString_Int` "" "+" 1 " Ghostlilly Seed"))))
    (:`2`
      (`TextRenderComponent.K2_SetText` _textrender (`KismetTextLibrary.Conv_StringToText` (`KismetStringLibrary.BuildString_Int` "" "+" 1 " Bushbow Seed"))))))

(event `self.ReceiveBeginPlay`
  ;[0 0.9023 1] Initializations
  (bind _returnvalue (`GameplayStatics.GetActorOfClass` "/Game/IBeWitching/Blueprints/Player.Player_C"))
  (set `self.PlayerRef` _returnvalue))

(event `self.ReceiveTick`
  (params (DeltaSeconds :type "Float (single-precision)"))
  (bind _textrender (`self.TextRender`))
  (bind _relativelocation (`SceneComponent.RelativeLocation` (`self.TextRender`)))
  ;[0 0.764 1] Tick
  (if (>= (.z _relativelocation) 100.0)
    (`self.K2_DestroyActor`)
    (else
      (`SceneComponent.K2_SetRelativeLocation` _textrender (`KismetMathLibrary.VLerp` _relativelocation (0.0 0.0 110.0) 0.01) false false)
      (`self.RotateTo` _textrender (`/Game/IBeWitching/Blueprints/Player.PlayerCam` (`self.PlayerRef`))))))

(event `RotateTo`
  (params (Origin :type "SceneComponent Object Reference") (Target :type "SceneComponent Object Reference"))
  (bind (_returnvalue_x _returnvalue_y _returnvalue_z) (`KismetMathLibrary.BreakVector` (`SceneComponent.K2_GetComponentLocation` Target)))
  (bind (_returnvalue_x_2 _returnvalue_y_2 _returnvalue_z_2) (`KismetMathLibrary.BreakVector` (`SceneComponent.K2_GetComponentLocation` Origin)))
  ;[1 0 0.007827] Rotate UI Function
  (`SceneComponent.K2_SetWorldRotation` Origin (`KismetMathLibrary.FindLookAtRotation` (`KismetMathLibrary.MakeVector` _returnvalue_x_2 _returnvalue_y_2 _returnvalue_z_2) (`KismetMathLibrary.MakeVector` _returnvalue_x _returnvalue_y_2 _returnvalue_z)) false false))

(fn `UserConstructionScript`)