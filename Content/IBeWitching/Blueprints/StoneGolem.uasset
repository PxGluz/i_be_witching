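; Stone Golem actor that the player carries with E and assigns to work areas, or leaves to chase nearby enemies.
; Tick drives animation, player-facing prompts and health bar, and carried, fetching or idle behavior.
; Fetching follows a runtime-built spline between work area and TouchStone, collecting and depositing items.
; When idle, it regenerates at its root, then lerps toward an enemy in range; death sends it back to recover.
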(event `Key|E`
  (params (Key :type "Key Structure"))
  ;[1 0.4788 0] PickUp/Drop Logic
  (:`Pressed`
    (if (`SceneComponent.IsVisible` (`self.PickUp`))
      (set `/Game/IBeWitching/Blueprints/Player.PickedUp` self (`self.PlayerRef`))
      (set `self.PickedUp` true)
      (`SceneComponent.SetVisibility` (`self.PickUp`) false false)
      (set `self.State` "Idle")
      (set `self.Speed` 0.0)
      (set `self.TargetEnemy` null)
      (elif (`SceneComponent.IsVisible` (`self.Drop`))
        (set `/Game/IBeWitching/Blueprints/Player.PickedUp` null (`self.PlayerRef`))
        (set `self.PickedUp` false)
        (`SceneComponent.SetVisibility` (`self.Drop`) false false)
        (set `self.State` "Idle")
        (set `self.Speed` 0.0)
        (`SceneComponent.K2_SetRelativeLocation` (`self.SkeletalMesh`) (0.0 0.0 0.0) false false)))))

(event `TakeDamage`
  (params (Amount :type "Float (double-precision)"))
  (bind _returnvalue (- (`self.Health`) Amount))
  ;[1 0 0.006631] Take Damage Function
  (if (<= _returnvalue 0.0)
    (set `self.Health` 0.0)
    (`self.Die`)
    (else
      (set `self.Health` _returnvalue))))

(event `Die`
  ;[1 0 0] Death Function
  (`SceneComponent.K2_SetRelativeLocation` (`self.SkeletalMesh`) (0.0 0.0 0.0) false true)
  (set `self.Respawning` true)
  (set `self.TargetEnemy` null)
  (set `self.Speed` 0.0)
  (set `self.State` "Idle")
  (set `self.PickedUp` false))

(event `RotateTo`
  (params (Origin :type "SceneComponent Object Reference") (Target :type "SceneComponent Object Reference"))
  (bind (_returnvalue_x _returnvalue_y _returnvalue_z) (`KismetMathLibrary.BreakVector` (`SceneComponent.K2_GetComponentLocation` Target)))
  (bind (_returnvalue_x_2 _returnvalue_y_2 _returnvalue_z_2) (`KismetMathLibrary.BreakVector` (`SceneComponent.K2_GetComponentLocation` Origin)))
  ;[1 0 0.007827] Rotate UI Function
  (`SceneComponent.K2_SetWorldRotation` Origin (`KismetMathLibrary.FindLookAtRotation` (`KismetMathLibrary.MakeVector` _returnvalue_x_2 _returnvalue_y_2 _returnvalue_z_2) (`KismetMathLibrary.MakeVector` _returnvalue_x _returnvalue_y_2 _returnvalue_z)) false false))

(event `AssignNewWork`
  (params (WorkArea :type "/Game/IBeWitching/Blueprints/PlantingGounds Object Reference"))
  ;[1 0 0.007827] Work Assigning
  (bind _output_get (set `self.WorkinArea` WorkArea))
  (`SplineComponent.SetSplinePoints` (`self.Spline`) (`|MakeArray` (`SceneComponent.K2_GetComponentLocation` (`Actor.RootComponent` _output_get)) (`SceneComponent.K2_GetComponentLocation` (`Actor.RootComponent` (`self.TouchStone`)))) "World" true)
  (set `self.State` "Fetching")
  (set `self.Speed` 300.0)
  (set `self.PickedUp` false)
  (set `/Game/IBeWitching/Blueprints/Player.PickedUp` null (`self.PlayerRef`))
  (set `self.DistanceOnSpline` 0.0)
  (set `self.PickingArea` false))

(event `self.ReceiveBeginPlay`
  ;[0 0.7962 1] Initializations
  (bind _returnvalue (`GameplayStatics.GetActorOfClass` "/Game/IBeWitching/Blueprints/TouchStone.TouchStone_C"))
  (set `self.TouchStone` _returnvalue)
  (bind _returnvalue_2 (`GameplayStatics.GetActorOfClass` "/Game/IBeWitching/Blueprints/Player.Player_C"))
  (set `self.PlayerRef` _returnvalue_2)
  (set `self.State` "Idle")
  (set `self.Speed` 0.0)
  (set `self.PickedUp` false)
  (set `self.Respawning` true))

(event `self.ReceiveTick`
  (params (DeltaSeconds :type "Float (single-precision)"))
  (bind _skeletalmesh (`self.SkeletalMesh`))
  (bind _health (`self.Health`))
  (bind _skeletalmesh_2 (`self.SkeletalMesh`))
  (bind _maxhealth (`self.MaxHealth`))
  (bind _pickup (`self.PickUp`))
  (bind _healthbar (`self.HealthBar`))
  (bind _skeletalmesh_3 (`self.SkeletalMesh`))
  (bind _drop (`self.Drop`))
  (bind _returnvalue (`SceneComponent.K2_GetComponentLocation` (`self.SkeletalMesh`)))
  (bind _capsulecomponent (`Character.CapsuleComponent` (`self.PlayerRef`)))
  (bind _playercam (`/Game/IBeWitching/Blueprints/Player.PlayerCam` (`self.PlayerRef`)))
  (bind _returnvalue_2 (`SceneComponent.K2_GetComponentLocation` (`Character.Mesh` (`self.TargetEnemy`))))
  (bind _returnvalue_3 (+ (* DeltaSeconds (`self.Speed`)) (`self.DistanceOnSpline`)))
  (bind _returnvalue_4 (`SplineComponent.GetTransformAtDistanceAlongSpline` (`self.Spline`) _returnvalue_3 "Local" false))
  ;[0 1 0.9937] Tick
  ;;[1 1 1] Animation Handling
  (if (> (`self.Speed`) 0.0)
    (if (not (`KismetStringLibrary.EqualEqual_StrStr` (`self.CurrentAnimation`) "Walking"))
      (`SkeletalMeshComponent.PlayAnimation` _skeletalmesh_2 "/Game/IBeWitching/Animations/WalkForwardAnim.WalkForwardAnim" true)
      (set `self.CurrentAnimation` "Walking"))
    (elif (`KismetStringLibrary.EqualEqual_StrStr` (`self.State`) "Idle")
      (if (not (`KismetStringLibrary.EqualEqual_StrStr` (`self.CurrentAnimation`) "Idle"))
        (`SkeletalMeshComponent.PlayAnimation` _skeletalmesh_2 "/Game/IBeWitching/Animations/Idle02Anim.Idle02Anim" true)
        (set `self.CurrentAnimation` "Idle"))
      (elif (not (`KismetStringLibrary.EqualEqual_StrStr` (`self.CurrentAnimation`) "Interacting"))
        (`SkeletalMeshComponent.PlayAnimation` _skeletalmesh_2 "/Game/IBeWitching/Animations/InteractAnim.InteractAnim" true)
        (set `self.CurrentAnimation` "Interacting"))))
  ;;[0 0.1384 1] HealthBar Logic
  (bind _asenemy_ui (cast `/Game/IBeWitching/Blueprints/EnemyUI` (`WidgetComponent.GetWidget` (`self.HealthBar`))))
  (set `ProgressBar.Percent` (/ (`self.Health`) (`self.MaxHealth`)) (`/Game/IBeWitching/Blueprints/EnemyUI.HealthBar` _asenemy_ui))
  (if (`self.PickedUp`)
    ;;[0.02731 1 0] PickedUp State
    (`SceneComponent.K2_SetWorldTransform` _skeletalmesh_3 (`KismetMathLibrary.MakeTransform` (+ (`SceneComponent.K2_GetComponentLocation` _capsulecomponent) (0.0 0.0 150.0)) (`SceneComponent.K2_GetComponentRotation` _capsulecomponent) (`SceneComponent.K2_GetComponentScale` _skeletalmesh_3)) false false)
    ;;;[0 0.07558 1] Drop UI Logic
    (if (`self.PickingArea`)
      (`SceneComponent.SetVisibility` _drop false false)
      (else
        (`SceneComponent.SetVisibility` _drop true false)
        (`self.EnableInput` (`GameplayStatics.GetPlayerController` 0))))
    (`self.RotateTo` (`self.Drop`) (`/Game/IBeWitching/Blueprints/Player.PlayerCam` (`self.PlayerRef`)))
    (`SceneComponent.SetVisibility` (`self.HealthBar`) false false)
    (else
      ;;[0.04055 1 0] Dropped State
      ;;;[0 0.0318 1] PickUp UI Logic
      (if (and (<= (`KismetMathLibrary.Vector_Distance` (`SceneComponent.K2_GetComponentLocation` (`Character.CapsuleComponent` (`self.PlayerRef`))) (`SceneComponent.K2_GetComponentLocation` (`self.SkeletalMesh`))) 100.0) (not (`KismetSystemLibrary.IsValid` (`/Game/IBeWitching/Blueprints/Player.PickedUp` (`self.PlayerRef`)))))
        (`SceneComponent.SetVisibility` _pickup true false)
        (`self.EnableInput` (`GameplayStatics.GetPlayerController` 0))
        (else
          (`SceneComponent.SetVisibility` _pickup false false)))
      (`self.RotateTo` (`self.PickUp`) _playercam)
      (`SceneComponent.SetVisibility` _healthbar true false)
      (`self.RotateTo` _healthbar _playercam)
      (if (`KismetStringLibrary.EqualEqual_StrStr` (`self.State`) "Fetching")
        ;;;[1 0 0.7782] Working State
        (if (>= (`self.DistanceOnSpline`) (/ (`SplineComponent.GetSplineLength` (`self.Spline`)) 2.0))
          (`/Game/IBeWitching/Blueprints/TouchStone.StoreItem` (`self.TouchStone`) (`self.CarriedType`) (`self.CarriedAmount`) self))
        (if (== (`self.DistanceOnSpline`) 0.0)
          (set `self.Speed` 0.0)
          (`/Game/IBeWitching/Blueprints/PlantingGounds.WorkerCollect` (`self.WorkinArea`) self))
        (set `self.DistanceOnSpline` _returnvalue_3)
        (`SceneComponent.K2_SetRelativeTransform` _skeletalmesh (`KismetMathLibrary.MakeTransform` (.location _returnvalue_4) (`KismetMathLibrary.MakeRotator` (.roll (.rotation _returnvalue_4)) (.pitch (.rotation _returnvalue_4)) (+ (.yaw (.rotation _returnvalue_4)) -90.0)) (`SceneComponent.RelativeScale3D` _skeletalmesh)) false false)
        (if (>= (`self.DistanceOnSpline`) (`SplineComponent.GetSplineLength` (`self.Spline`)))
          (set `self.DistanceOnSpline` 0.0))
        (else
          ;;;[1 0 0.8912] Idle/Picking State
          (if (or (`self.Respawning`) (not (`KismetSystemLibrary.IsValid` (`self.TargetEnemy`))))
            (set `self.Speed` 0.0)
            (`SceneComponent.K2_SetRelativeLocation` (`self.SkeletalMesh`) (0.0 0.0 0.0) false true :!label _label)
            (set `self.Health` (`KismetMathLibrary.Lerp` _health _maxhealth 0.005))
            (if (`KismetMathLibrary.NearlyEqual_FloatFloat` _health _maxhealth 1.0)
              (set `self.Respawning` false)
              (set `self.Health` _maxhealth)
              (bind _outactors (`GameplayStatics.GetAllActorsOfClass` "/Game/IBeWitching/Blueprints/Enemy.Enemy_C"))
              (for _array_element _outactors
                (if (<= (`KismetMathLibrary.Vector_Distance` (`SceneComponent.K2_GetComponentLocation` (`Character.Mesh` _array_element)) (`SceneComponent.K2_GetComponentLocation` (`self.DefaultSceneRoot`))) 500.0)
                  (set `self.TargetEnemy` _array_element))))
            (else
              (set `self.Speed` 1.0)
              (`/Engine/EditorBlueprintResources/StandardMacros.IsValid` (`self.TargetEnemy`)
                (:`Is Valid`
                  (`SceneComponent.K2_SetWorldLocation` (`self.SkeletalMesh`) (`KismetMathLibrary.VLerp` _returnvalue _returnvalue_2 0.02) false false)
                  (`SceneComponent.K2_SetWorldRotation` (`self.SkeletalMesh`) (`KismetMathLibrary.FindLookAtRotation` _returnvalue_2 _returnvalue) false false))
                (:`Is Not Valid`
                  (set `self.TargetEnemy` null)
                  (goto _label))))))))))

(fn `UserConstructionScript`)