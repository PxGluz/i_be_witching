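; Enemy pawn that chases and damages whichever is nearest: a living Player or a tagged StoneGolem.
; Each tick it picks the closest target, moves via AIMoveTo and tints its spotlight yellow for golems, red otherwise.
; Capsule overlaps deal damage, also taking damage from golems, with temporary Block responses and delays spacing out hits.
; It destroys itself at zero health and updates a widget health bar that rotates toward the player camera.
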(event `RotateTo`
  (params (Origin :type "SceneComponent Object Reference") (Target :type "SceneComponent Object Reference"))
  (bind (_returnvalue_x _returnvalue_y _returnvalue_z) (`KismetMathLibrary.BreakVector` (`SceneComponent.K2_GetComponentLocation` Target)))
  (bind (_returnvalue_x_2 _returnvalue_y_2 _returnvalue_z_2) (`KismetMathLibrary.BreakVector` (`SceneComponent.K2_GetComponentLocation` Origin)))
  ;[1 0 0.007827] Rotate UI Function
  (`SceneComponent.K2_SetWorldRotation` Origin (`KismetMathLibrary.FindLookAtRotation` (`KismetMathLibrary.MakeVector` _returnvalue_x_2 _returnvalue_y_2 _returnvalue_z_2) (`KismetMathLibrary.MakeVector` _returnvalue_x _returnvalue_y_2 _returnvalue_z)) false false))

(event `self.CapsuleComponent.OnComponentBeginOverlap`
  (params (OverlappedComponent :type "PrimitiveComponent Object Reference") (OtherActor :type "Actor Object Reference") (OtherComp :type "PrimitiveComponent Object Reference") (OtherBodyIndex :type Integer) (bFromSweep :type Boolean) (SweepResult :type "HitResult Structure (by ref)"))
  (bind _damage (`self.Damage`))
  (bind _capsulecomponent (`self.CapsuleComponent`))
  (bind _asplayer (cast `/Game/IBeWitching/Blueprints/Player` OtherActor)
    (:`then`
      (`/Game/IBeWitching/Blueprints/Player.TakeDamage` _asplayer _damage)
      (`PrimitiveComponent.SetCollisionResponseToChannel` _capsulecomponent "ECC_Pawn" "ECR_Block")
      (`KismetSystemLibrary.Delay` 1.0)
      (`PrimitiveComponent.SetCollisionResponseToChannel` _capsulecomponent "ECC_Pawn" "ECR_Overlap"))
    (:`CastFailed`
      (bind _asstone_golem (cast `/Game/IBeWitching/Blueprints/StoneGolem` OtherActor))
      (`self.TakeDamage` (`/Game/IBeWitching/Blueprints/StoneGolem.Damage` _asstone_golem))
      (if (and (`self.CanDamage`) (> (`self.Health`) 0.0))
        (set `self.CanDamage` false)
        (`/Game/IBeWitching/Blueprints/StoneGolem.TakeDamage` _asstone_golem _damage)
        (`PrimitiveComponent.SetCollisionResponseToChannel` _capsulecomponent "ECC_WorldDynamic" "ECR_Block")
        (`KismetSystemLibrary.Delay` 1.0)
        (`PrimitiveComponent.SetCollisionResponseToChannel` _capsulecomponent "ECC_WorldDynamic" "ECR_Overlap")
        (set `self.CanDamage` true)))))

(event `TakeDamage`
  (params (Amount :type "Float (double-precision)"))
  (bind _returnvalue (- (`self.Health`) Amount))
  ;[1 0 0.006631] Take Damage Function
  (if (<= _returnvalue 0.0)
    (`self.K2_DestroyActor`)
    (else
      (set `self.Health` _returnvalue))))

(event `self.ReceiveBeginPlay`
  (bind _returnvalue (`GameplayStatics.GetActorOfClass` "/Game/IBeWitching/Blueprints/Player.Player_C"))
  (set `self.PlayerRef` _returnvalue))

(event `self.ReceiveTick`
  (params (DeltaSeconds :type "Float (single-precision)"))
  (bind _playerref (`self.PlayerRef`))
  (bind _spotlight (`self.SpotLight`))
  (bind _actortofollow (`self.ActorToFollow`))
  (bind _enemyhealth (`self.EnemyHealth`))
  (bind _asenemy_ui (cast `/Game/IBeWitching/Blueprints/EnemyUI` (`WidgetComponent.GetWidget` _enemyhealth))
    (:`then`
      (set `ProgressBar.Percent` (/ (`self.Health`) (`self.MaxHealth`)) (`/Game/IBeWitching/Blueprints/EnemyUI.HealthBar` _asenemy_ui)))
    (:`CastFailed`
      _))
  (bind _asplayer (cast `/Game/IBeWitching/Blueprints/Player` (`self.PlayerRef`))
    (:`then`
      (`self.RotateTo` _enemyhealth (`/Game/IBeWitching/Blueprints/Player.PlayerCam` _asplayer)))
    (:`CastFailed`
      _))
  (bind _outactors (`GameplayStatics.GetAllActorsWithTag` "Golem"))
  (bind _output_get (set `self.Out Actors` _outactors))
  (bind _asplayer_2 (cast `/Game/IBeWitching/Blueprints/Player` _playerref)
    (:`then`
      (if (not (`/Game/IBeWitching/Blueprints/Player.Dead` _asplayer_2))
        (`KismetArrayLibrary.Array_Add` _output_get _playerref)))
    (:`CastFailed`
      _))
  (set `self.ActorDistance` 100000.0)
  (for _array_element (`self.Out Actors`)
    (bind _asstone_golem (cast `/Game/IBeWitching/Blueprints/StoneGolem` _array_element)
      (:`then`
        (bind _returnvalue (`KismetMathLibrary.Vector_Distance` (`self.K2_GetActorLocation`) (`SceneComponent.K2_GetComponentLocation` (`/Game/IBeWitching/Blueprints/StoneGolem.SkeletalMesh` _asstone_golem))))
        (if (< _returnvalue (`self.ActorDistance`))
          (set `self.ActorToFollow` _array_element)
          (set `self.ActorDistance` _returnvalue)))
      (:`CastFailed`
        (bind _returnvalue_2 (`KismetMathLibrary.Vector_Distance` (`self.K2_GetActorLocation` _array_element) (`self.K2_GetActorLocation`)))
        (if (< _returnvalue_2 (`self.ActorDistance`))
          (set `self.ActorToFollow` _array_element)
          (set `self.ActorDistance` _returnvalue_2)))))
  (bind _asstone_golem_2 (cast `/Game/IBeWitching/Blueprints/StoneGolem` _actortofollow)
    (:`then`
      (`LightComponent.SetLightColor` _spotlight (struct :`R` 1.0 :`G` 0.933874 :`A` 1.0) true)
      (`|AIMoveTo` self (`SceneComponent.K2_GetComponentLocation` (`/Game/IBeWitching/Blueprints/StoneGolem.SkeletalMesh` _asstone_golem_2)) null 0.0))
    (:`CastFailed`
      (`LightComponent.SetLightColor` _spotlight (struct :`R` 1.0 :`A` 1.0) true)
      (`|AIMoveTo` self (0.0 0.0 0.0) _actortofollow 0.0))))

(fn `UserConstructionScript`)