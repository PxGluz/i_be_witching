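; Planting plot actor that holds up to four tiers of PlantBP child actors and a cache count of the selected plant.
; BeginPlay activates the first tier; R reveals each next one with a higher SlotSpeed and raises MaxCache.
; E stores the cache in the TouchStone or assigns the carried worker, while WorkerCollect hands it to workers.
; Tick toggles prompts and enables input by player proximity, updates the count label and yaws widgets toward the camera.
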(event `Key|R`
  (params (Key :type "Key Structure"))
  (bind _level2 (`self.Level2`))
  (bind _level3 (`self.Level3`))
  (bind _level4 (`self.Level4`))
  ;[0.97 1 0.3198] Input Handling
  ;;[1 0.4267 0] Upgrade Function
  (:`Pressed`
    (if (`SceneComponent.IsVisible` (`self.Upgrade`))
      (if (`SceneComponent.IsVisible` _level2)
        (if (`SceneComponent.IsVisible` _level3)
          (if (not (`SceneComponent.IsVisible` _level4))
            (`SceneComponent.SetVisibility` _level4 true false)
            (bind _asplant_bp (cast `/Game/IBeWitching/Blueprints/PlantBP` (`ChildActorComponent.ChildActor` _level4)))
            (`/Game/IBeWitching/Blueprints/PlantBP.SetPlant` _asplant_bp self (`self.SelectedPlant`) 0.5)
            (set `self.MaxCache` (+ (`self.MaxCache`) 5)))
          (else
            (`SceneComponent.SetVisibility` _level3 true false)
            (bind _asplant_bp_2 (cast `/Game/IBeWitching/Blueprints/PlantBP` (`ChildActorComponent.ChildActor` _level3)))
            (`/Game/IBeWitching/Blueprints/PlantBP.SetPlant` _asplant_bp_2 self (`self.SelectedPlant`) 0.3)
            (set `self.MaxCache` (+ (`self.MaxCache`) 5))))
        (else
          (`SceneComponent.SetVisibility` _level2 true false)
          (bind _asplant_bp_3 (cast `/Game/IBeWitching/Blueprints/PlantBP` (`ChildActorComponent.ChildActor` _level2)))
          (`/Game/IBeWitching/Blueprints/PlantBP.SetPlant` _asplant_bp_3 self (`self.SelectedPlant`) 0.15)
          (set `self.MaxCache` (+ (`self.MaxCache`) 5)))))))

(event `WorkerCollect`
  (params (Worker :type "/Game/IBeWitching/Blueprints/StoneGolem Object Reference"))
  ;[1 0 0.02708] Worker Collection
  (set `/Game/IBeWitching/Blueprints/StoneGolem.CarriedType` (`self.SelectedPlant`) Worker)
  (set `/Game/IBeWitching/Blueprints/StoneGolem.CarriedAmount` (+ (`self.CacheCount`) (`/Game/IBeWitching/Blueprints/StoneGolem.CarriedAmount` Worker)) Worker)
  (if (> (`self.CacheCount`) 0)
    (set `/Game/IBeWitching/Blueprints/StoneGolem.Speed` 300.0 Worker)
    (set `self.CacheCount` 0)))

(event `Key|E`
  (params (Key :type "Key Structure"))
  ;[0.97 1 0.3198] Input Handling
  ;;[1 0.4142 0] Manual Collection Function
  (:`Pressed`
    (if (`SceneComponent.IsVisible` (`self.Collect`))
      (`/Game/IBeWitching/Blueprints/TouchStone.StoreItem` (`self.TouchStone`) (`self.SelectedPlant`) (`self.CacheCount`) null)
      (set `self.CacheCount` 0)
      (elif (`SceneComponent.IsVisible` (`self.Worker`))
        (`/Game/IBeWitching/Blueprints/StoneGolem.AssignNewWork` (`/Game/IBeWitching/Blueprints/Player.PickedUp` (`self.PlayerReference`)) self)
        (`SceneComponent.SetVisibility` (`self.Worker`) false false)))))

(event `self.ReceiveBeginPlay`
  (bind _level1 (`self.Level1`))
  ;[0 0.901 1] Initializations
  (bind _asplant_bp (cast `/Game/IBeWitching/Blueprints/PlantBP` (`ChildActorComponent.ChildActor` _level1)))
  (`/Game/IBeWitching/Blueprints/PlantBP.SetPlant` _asplant_bp self (`self.SelectedPlant`) 0.1)
  (`SceneComponent.SetVisibility` _level1 true true)
  (bind _returnvalue (`GameplayStatics.GetActorOfClass` "/Game/IBeWitching/Blueprints/Player.Player_C"))
  (set `self.PlayerReference` _returnvalue)
  (bind _returnvalue_2 (`GameplayStatics.GetActorOfClass` "/Game/IBeWitching/Blueprints/TouchStone.TouchStone_C"))
  (set `self.TouchStone` _returnvalue_2))

(event `RotateTo`
  (params (Origin :type "SceneComponent Object Reference") (Target :type "SceneComponent Object Reference"))
  (bind (_returnvalue_x _returnvalue_y _returnvalue_z) (`KismetMathLibrary.BreakVector` (`SceneComponent.K2_GetComponentLocation` Target)))
  (bind (_returnvalue_x_2 _returnvalue_y_2 _returnvalue_z_2) (`KismetMathLibrary.BreakVector` (`SceneComponent.K2_GetComponentLocation` Origin)))
  ;[0 0.8835 1] Tick
  ;;[1 0 0.04149] UI Rotation Function
  (`SceneComponent.K2_SetWorldRotation` Origin (`KismetMathLibrary.FindLookAtRotation` (`KismetMathLibrary.MakeVector` _returnvalue_x_2 _returnvalue_y_2 _returnvalue_z_2) (`KismetMathLibrary.MakeVector` _returnvalue_x _returnvalue_y_2 _returnvalue_z)) false false))

(event `self.ReceiveTick`
  (params (DeltaSeconds :type "Float (single-precision)"))
  (bind _upgrade (`self.Upgrade`))
  (bind _collect (`self.Collect`))
  (bind _worker (`self.Worker`))
  (bind _count (`self.Count`))
  (bind _playercam (`/Game/IBeWitching/Blueprints/Player.PlayerCam` (`self.PlayerReference`)))
  ;[0 0.8835 1] Tick
  (bind _asplant_bp (cast `/Game/IBeWitching/Blueprints/PlantBP` (`ChildActorComponent.ChildActor` (`self.Level1`))))
  ;;[0 1 0.04119] Player Detection
  (if (<= (`KismetMathLibrary.Vector_Distance` (`SceneComponent.K2_GetComponentLocation` (`Character.CapsuleComponent` (`self.PlayerReference`))) (`SceneComponent.K2_GetComponentLocation` (`self.DefaultSceneRoot`))) 350.0)
    ;;[0.2014 0.2092 1] UI Logic
    (if (`KismetSystemLibrary.IsValid` (`/Game/IBeWitching/Blueprints/Player.PickedUp` (`self.PlayerReference`)))
      (`SceneComponent.SetVisibility` _upgrade false false)
      (`SceneComponent.SetVisibility` _collect false false)
      (`SceneComponent.SetVisibility` _worker true false)
      (set `/Game/IBeWitching/Blueprints/StoneGolem.PickingArea` true (`/Game/IBeWitching/Blueprints/Player.PickedUp` (`self.PlayerReference`)))
      (else
        (`SceneComponent.SetVisibility` _upgrade true false)
        (`SceneComponent.SetVisibility` _collect true false)
        (`SceneComponent.SetVisibility` _worker false false)))
    (`self.EnableInput` (`GameplayStatics.GetPlayerController` 0))
    (else
      (if (and (`KismetSystemLibrary.IsValid` (`/Game/IBeWitching/Blueprints/Player.PickedUp` (`self.PlayerReference`))) (`SceneComponent.IsVisible` (`self.Worker`)))
        (set `/Game/IBeWitching/Blueprints/StoneGolem.PickingArea` false (`/Game/IBeWitching/Blueprints/Player.PickedUp` (`self.PlayerReference`))))
      (`SceneComponent.SetVisibility` _upgrade false false)
      (`SceneComponent.SetVisibility` _collect false false)
      (`SceneComponent.SetVisibility` _worker false false)))
  ;;[0.284 0.2499 1] UI Rotation
  (`TextRenderComponent.K2_SetText` _count (`KismetTextLibrary.Conv_StringToText` (`KismetStringLibrary.Concat_StrStr` (`KismetStringLibrary.Concat_StrStr` (`KismetStringLibrary.Conv_IntToString` (`self.CacheCount`)) " ") (`KismetStringLibrary.Concat_StrStr` (`KismetStringLibrary.Replace` (`KismetSystemLibrary.GetObjectName` (`StaticMeshComponent.StaticMesh` (`/Game/IBeWitching/Blueprints/PlantBP.Model` _asplant_bp))) "_" " ") "s Stored"))))
  (`self.RotateTo` _count _playercam)
  (`self.RotateTo` (`self.Collect`) _playercam)
  (`self.RotateTo` (`self.Upgrade`) _playercam)
  (`self.RotateTo` (`self.Worker`) _playercam)
  (if (`SceneComponent.IsVisible` (`self.Level4`))
    (`SceneComponent.SetVisibility` (`self.Upgrade`) false false)))

(fn `UserConstructionScript`)